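; Enemy actor that shuttles back and forth between two positions and ends the game when it touches the player.
; BeginPlay records the actor location as the start, then Move slides the static mesh toward EndPosition with MoveComponentTo, swapping targets and calling itself again to loop.
; StartPosition is a world location, but the move treats targets as relative locations.
; An overlap with a Player calls its GameOver.
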(event Custom|Move
  ;[1 1 1] Enemy Movement
  (Components|MoveComponentTo (Variables|Default|GetStaticMesh) (Variables|Default|GettargetPosition) "0, 0, 0" false false (Variables|Default|GetmoveSpeed) false)
  (if (Utilities|Operators|EqualEqual (Variables|Default|GettargetPosition) (Variables|Default|GetstartPosition) 0.001)
    (Variables|Default|SettargetPosition (Variables|Default|GetendPosition))
    (CallFunction|Move)
    (else
      (Variables|Default|SettargetPosition (Variables|Default|GetstartPosition))
      (CallFunction|Move))))

(event EventBeginPlay
  ;[1 1 1] Enemy Movement
  (Variables|Default|SetstartPosition (Transformation|GetActorLocation))
  (Variables|Default|SettargetPosition (Variables|Default|GetendPosition))
  (CallFunction|Move))

(event Collision|EventActorBeginOverlap
  (params (OtherActor :type Actor%20Object%20Reference))
  ;[1 1 1] Player Overlap
  (bind _asplayer (Utilities|Casting|CastToPlayer OtherActor))
  (Default|GameOver _asplayer))

(fn ConstructionScript)