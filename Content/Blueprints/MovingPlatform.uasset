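; A moving platform that shuttles its static mesh endlessly between a start point and an offset end point.
; On BeginPlay it derives both points from the actor's transform and OffSet, keeping the starting rotation.
; A self-calling Move event runs MoveComponentTo, using those world values as relative targets and MoveSpeed as duration.
; After each move it flips the target and repeats, with no Tick or Timeline.
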(event Custom|Move
  (Components|MoveComponentTo (Variables|Default|GetStaticMesh) (Variables|Default|GettargetPosition) (Variables|Default|GetRotation) false false (Variables|Default|GetmoveSpeed) false)
  (if (Utilities|Operators|EqualEqual (Variables|Default|GettargetPosition) (Variables|Default|GetstartPosition) 0.001)
    (Variables|Default|SettargetPosition (Variables|Default|GetendPosition))
    (CallFunction|Move)
    (else
      (Variables|Default|SettargetPosition (Variables|Default|GetstartPosition))
      (CallFunction|Move))))

(event EventBeginPlay
  (bind _output_get (Variables|Default|SetstartTransfrom (Transformation|GetActorTransform)))
  (Variables|Default|SetRotation (.rotation _output_get))
  (Variables|Default|SetstartPosition (.location _output_get))
  (Variables|Default|SetendPosition (+ (Variables|Default|GetoffSet) (Variables|Default|GetstartPosition)))
  (Variables|Default|SettargetPosition (Variables|Default|GetendPosition))
  (CallFunction|Move))

(fn ConstructionScript)